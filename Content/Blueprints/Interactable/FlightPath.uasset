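; FlightPath is a spline actor that lays out a flight route with targets and path markers.
; The construction script walks the spline twice, spawning child actor components at separate configurable spacings for the target and marker classes.
; Targets inherit the spline's scale at each point, while markers are forced to unit world scale.
; Placement starts one spacing in from the spline's start, and the event graph has no logic.
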(fn `AddMarkers`
  (locals (distance :type "Float (double-precision)"))
  (while (< (`local.distance`) (`SplineComponent.GetSplineLength` (`self.Spline`)))
    (bind _output_get (set `local.distance` (+ (`local.distance`) (`self.markerSpacing`))))
    (bind _returnvalue (`AddComponent|NODE_AddChildActorComponent-3` :`RelativeTransform` (`SplineComponent.GetTransformAtDistanceAlongSpline` (`self.Spline`) _output_get "Local" false)))
    (`ChildActorComponent.SetChildActorClass` _returnvalue (`self.markerClass`))
    (`SceneComponent.SetWorldScale3D` _returnvalue (1.0 1.0 1.0))))

(fn `AddTargets`
  (locals (Distance :type "Float (double-precision)"))
  (while (< (`local.distance`) (`SplineComponent.GetSplineLength` (`self.Spline`)))
    (bind _output_get (set `local.distance` (+ (`local.distance`) (`self.targetSpacing`))))
    (bind _returnvalue (`AddComponent|NODE_AddChildActorComponent-1` :`RelativeTransform` (`SplineComponent.GetTransformAtDistanceAlongSpline` (`self.Spline`) _output_get "Local" true)))
    (`ChildActorComponent.SetChildActorClass` _returnvalue (`self.targetMarkerClass`))))

(fn `UserConstructionScript`
  (`self.AddTargets`)
  (`self.AddMarkers`))